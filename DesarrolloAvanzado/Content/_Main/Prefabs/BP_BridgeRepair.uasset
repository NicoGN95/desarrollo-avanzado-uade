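; A bridge repair point that the player fixes by bringing a BP_MetalSheet into its Box trigger.
; It starts with the Repaired component hidden and non-colliding, then reveals it and hides the overlapping sheet.
; The Acho event undoes a repair, attaching the sheet to the player's Hand and marking it held, but leaves IsRepaired true.
; The game instance's ItemStored comes from GetActorOfClass, not the cached sheet reference.
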(event `self.ReceiveBeginPlay`
  (bind _repaired (`self.Repaired`))
  ;[1 1 1] Awake
  (bind _asthird_person_character (cast `/Game/ThirdPersonBP/Blueprints/ThirdPersonCharacter` (`GameplayStatics.GetPlayerCharacter` 0)))
  (set `self.player` _asthird_person_character)
  (bind _asbpgi_instance (cast `/Game/_BP/BPGI_Instance` (`GameplayStatics.GetGameInstance`)))
  (set `self.As BPGI Instance` _asbpgi_instance)
  (`SceneComponent.SetVisibility` _repaired false false)
  (`PrimitiveComponent.SetCollisionEnabled` _repaired "NoCollision")
  (`ActorComponent.SetComponentTickEnabled` _repaired false))

(event `self.Box.OnComponentBeginOverlap`
  (params (OverlappedComponent :type "PrimitiveComponent Object Reference") (OtherActor :type "Actor Object Reference") (OtherComp :type "PrimitiveComponent Object Reference") (OtherBodyIndex :type Integer) (bFromSweep :type Boolean) (SweepResult :type "HitResult Structure (by ref)"))
  (bind _as_bp_metal_sheet (`self.As BP Metal Sheet`))
  (bind _repaired (`self.Repaired`))
  ;[1 1 1] OverlapCollision
  (bind _asbp_metal_sheet (cast `/Game/_Main/Prefabs/BP_MetalSheet` OtherActor))
  (set `self.As BP Metal Sheet` _asbp_metal_sheet)
  (`SceneComponent.SetVisibility` _repaired true false)
  (`PrimitiveComponent.SetCollisionEnabled` _repaired "QueryAndPhysics")
  (`ActorComponent.SetComponentTickEnabled` _repaired true)
  (`SceneComponent.SetVisibility` (`Actor.RootComponent` _as_bp_metal_sheet) false false)
  (`PrimitiveComponent.SetCollisionEnabled` (`StaticMeshActor.StaticMeshComponent` _as_bp_metal_sheet) "PhysicsOnly")
  (set `self.IsRepaired` true))

(event `/Game/Interfaces/BPI_I.acho`
  (bind _repaired (`self.Repaired`))
  (bind _as_bp_metal_sheet (`self.As BP Metal Sheet`))
  (bind _as_bp_metal_sheet_2 (`self.As BP Metal Sheet`))
  (bind _hand (`/Game/ThirdPersonBP/Blueprints/ThirdPersonCharacter.hand` (`self.player`)))
  (if (`self.IsRepaired`)
    (`SceneComponent.SetVisibility` _repaired false false)
    (`PrimitiveComponent.SetCollisionEnabled` _repaired "NoCollision")
    (`ActorComponent.SetComponentTickEnabled` _repaired false)
    (`SceneComponent.SetVisibility` (`Actor.RootComponent` _as_bp_metal_sheet) true false)
    (`PrimitiveComponent.SetCollisionEnabled` (`StaticMeshActor.StaticMeshComponent` _as_bp_metal_sheet) "QueryAndPhysics")
    (`self.K2_SetActorLocation` _as_bp_metal_sheet_2 (`SceneComponent.K2_GetComponentLocation` _hand) false false)
    (`self.SetActorEnableCollision` _as_bp_metal_sheet_2 false)
    (`PrimitiveComponent.SetSimulatePhysics` (`StaticMeshActor.StaticMeshComponent` _as_bp_metal_sheet_2) false)
    (`self.K2_AttachToComponent` _as_bp_metal_sheet_2 _hand "None" "SnapToTarget" "SnapToTarget" "SnapToTarget" true)
    (bind _returnvalue (`GameplayStatics.GetActorOfClass` "/Game/_Main/Prefabs/BP_MetalSheet.BP_MetalSheet_C"))
    (set `/Game/_BP/BPGI_Instance.ItemStored` _returnvalue (`self.As BPGI Instance`))
    (set `/Game/ThirdPersonBP/Blueprints/ThirdPersonCharacter.isHoldingAnItem?` true (`self.player`))))

(fn `UserConstructionScript`)