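; BP_Comida is a food item that feeds the player by a set food amount.
; Its Acho event passes that amount to the third-person player character's TakeFood, then destroys the actor.
; A separate Interact function overwrites Hunger on the game instance with the same amount and returns false, leaving the item in the world.
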(event `/Game/Interfaces/BPI_I.acho`
  (bind _asthird_person_character (cast `/Game/ThirdPersonBP/Blueprints/ThirdPersonCharacter` (`GameplayStatics.GetPlayerCharacter` 0)))
  (`/Game/ThirdPersonBP/Blueprints/ThirdPersonCharacter.TakeFood` _asthird_person_character (`self.FoodAmmount`))
  (`self.K2_DestroyActor`))

(fn `Interact`
  (returns (`Did_Interact?` :type Boolean))
  (bind _asbpgi_instance (cast `/Game/_BP/BPGI_Instance` (`GameplayStatics.GetGameInstance`)))
  (bind _output_get (set `self.As BPGI Instance` _asbpgi_instance))
  (set `/Game/_BP/BPGI_Instance.Hunger` (`self.FoodAmmount`) _output_get)
  (return false))

(fn `UserConstructionScript`)