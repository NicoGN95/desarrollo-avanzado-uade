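; BP_TestMetalSheet is a test metal sheet item that the player can pick up and hold.
; On BeginPlay it caches the ThirdPersonCharacter and the BPGI_Instance game instance.
; The Acho event, if the player's hands are free, disables collision and physics, snaps to the Hand component and sets IsHoldingAnItem.
; It stores the result of GetActorOfClass, not self, in ItemStored, so another sheet instance may be recorded.
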(event `self.ReceiveBeginPlay`
  ;[1 1 1] Awake
  (bind _asthird_person_character (cast `/Game/ThirdPersonBP/Blueprints/ThirdPersonCharacter` (`GameplayStatics.GetPlayerCharacter` 0)))
  (set `self.player` _asthird_person_character)
  (bind _asbpgi_instance (cast `/Game/_BP/BPGI_Instance` (`GameplayStatics.GetGameInstance`)))
  (set `self.As BPGI Instance` _asbpgi_instance))

(event `/Game/Interfaces/BPI_I.acho`
  (bind _hand (`/Game/ThirdPersonBP/Blueprints/ThirdPersonCharacter.hand` (`self.player`)))
  ;[1 1 1] Interaction
  (if (not (`/Game/ThirdPersonBP/Blueprints/ThirdPersonCharacter.isHoldingAnItem?` (`self.player`)))
    (`self.K2_SetActorLocation` (`SceneComponent.K2_GetComponentLocation` _hand))
    (`self.SetActorEnableCollision` false)
    (`PrimitiveComponent.SetSimulatePhysics` (`self.Cube`) false)
    (`self.K2_AttachToComponent` _hand "None" "SnapToTarget" "SnapToTarget" "SnapToTarget")
    (bind _returnvalue (`GameplayStatics.GetActorOfClass` "BP_TestMetalSheet_C"))
    (set `/Game/_BP/BPGI_Instance.ItemStored` _returnvalue (`self.As BPGI Instance`))
    (set `/Game/ThirdPersonBP/Blueprints/ThirdPersonCharacter.isHoldingAnItem?` true (`self.player`))))

(fn `UserConstructionScript`)